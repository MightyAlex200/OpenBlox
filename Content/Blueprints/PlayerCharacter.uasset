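; Player character Blueprint with jumping, yaw-relative movement and a zoomable camera that switches between third-person and first-person control.
; The mouse wheel adjusts the clamped spring arm length, enabling rotation lag whenever the arm is extended.
; When zoomed out, the cursor shows and looking requires holding right mouse.
; At zero arm length, the cursor hides and mouse movement turns the view freely.
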(event `InputAction|Jump`
  (params (Key :type "Key Structure" :default "AnyKey"))
  (:`Pressed`
    (`self.Jump`)))

(event `InputAxis|Forward`
  (params (AxisValue :type "Float (single-precision)"))
  (bind (_returnvalue_roll _returnvalue_pitch _returnvalue_yaw) (`KismetMathLibrary.BreakRotator` (`self.GetControlRotation`)))
  ;[1 1 1] Movement
  (`self.AddMovementInput` (`KismetMathLibrary.GetForwardVector` (`KismetMathLibrary.MakeRotator` 0.0 0.0 _returnvalue_yaw)) AxisValue))

(event `InputAxis|Right`
  (params (AxisValue :type "Float (single-precision)"))
  (bind (_returnvalue_roll _returnvalue_pitch _returnvalue_yaw) (`KismetMathLibrary.BreakRotator` (`self.GetControlRotation`)))
  ;[1 1 1] Movement
  (`self.AddMovementInput` (`KismetMathLibrary.GetRightVector` (`KismetMathLibrary.MakeRotator` 0.0 0.0 _returnvalue_yaw)) AxisValue))

(event `InputAxisKey|MouseY`
  (params (AxisValue :type "Float (single-precision)"))
  ;[1 1 1] Mouse Y
  (if (> (`SpringArmComponent.TargetArmLength` (`self.SpringArm`)) 0.0)
    (if (`PlayerController.IsInputKeyDown` (`GameplayStatics.GetPlayerController` 0) "RightMouseButton")
      (`self.AddControllerPitchInput` (* AxisValue -1.0) :!label _label))
    (else
      (goto _label))))

(event `InputAxisKey|MouseWheelAxis`
  (params (AxisValue :type "Float (single-precision)"))
  (bind _springarm (`self.SpringArm`))
  ;[1 1 1] Mouse Scroll
  (bind _output_get (set `SpringArmComponent.TargetArmLength` (`KismetMathLibrary.FMin` (`KismetMathLibrary.FMax` (+ (* AxisValue -25.0) (`SpringArmComponent.TargetArmLength` _springarm))) 1500.0) _springarm))
  (set `SpringArmComponent.bEnableCameraRotationLag` (> _output_get 0.0) (`self.SpringArm`)))

(event `InputAxisKey|MouseX`
  (params (AxisValue :type "Float (single-precision)"))
  ;[1 1 1] Mouse X
  (if (> (`SpringArmComponent.TargetArmLength` (`self.SpringArm`)) 0.0)
    (if (`PlayerController.IsInputKeyDown` (`GameplayStatics.GetPlayerController` 0) "RightMouseButton")
      (`self.AddControllerYawInput` AxisValue :!label _label_2))
    (else
      (goto _label_2))))

(event `self.ReceiveTick`
  (params (DeltaSeconds :type "Float (single-precision)"))
  ;[1 1 1] Tick
  (set `PlayerController.bShowMouseCursor` (> (`SpringArmComponent.TargetArmLength` (`self.SpringArm`)) 0.0) (`GameplayStatics.GetPlayerController` 0)))

(fn `UserConstructionScript`)