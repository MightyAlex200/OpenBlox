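; Base item Blueprint for pickups that the player collects on collision and stores in an inventory.
; On Hit, it casts to PlayerCharacter, adds itself to that Items array if absent, then hides and disables collision instead of destroying itself.
; Show, Hide, StartCollision and StopCollision toggle visibility and static mesh collision.
; Use is a placeholder that prints a warning that no use function exists.
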(event `self.ReceiveHit`
  (params (MyComp :type "PrimitiveComponent Object Reference") (Other :type "Actor Object Reference") (OtherComp :type "PrimitiveComponent Object Reference") (bSelfMoved :type Boolean) (HitLocation :type "Vector Structure") (HitNormal :type "Vector Structure") (NormalImpulse :type "Vector Structure") (Hit :type "HitResult Structure (by ref)"))
  (bind _asplayer_character (cast `/Game/Character/PlayerCharacter` Other))
  (bind _items (`/Game/Character/PlayerCharacter.Items` _asplayer_character))
  (if (== (`KismetArrayLibrary.Array_Find` _items self) -1)
    (`KismetArrayLibrary.Array_Add` _items self)
    (`self.Hide`)
    (`self.StopCollision`)))

(fn `Hide`
  (`self.SetActorHiddenInGame` true))

(fn `Show`
  (`self.SetActorHiddenInGame` false))

(fn `StartCollision`
  (for _array_element (`self.K2_GetComponentsByClass` "/Script/Engine.StaticMeshComponent")
    (`PrimitiveComponent.SetCollisionEnabled` _array_element "QueryAndPhysics")))

(fn `StopCollision`
  (for _array_element (`self.K2_GetComponentsByClass` "/Script/Engine.StaticMeshComponent")
    (`PrimitiveComponent.SetCollisionEnabled` _array_element "NoCollision")))

(fn `Use`
  (`KismetSystemLibrary.PrintString` "This item has not been given a \"use\" function. Please create one."))

(fn `UserConstructionScript`)